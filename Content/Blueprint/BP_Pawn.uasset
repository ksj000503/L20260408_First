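; BP_Pawn is a flying pawn, apparently a propeller plane, that constantly moves along its forward vector.
; Pitch and Roll axis inputs apply frame-rate-independent local rotation, steering the direction of that movement.
; A RotatePropeller helper spins a given component around its local roll axis, but its left and right propeller calls are disconnected, so they never run.
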(event `self.ReceiveTick`
  (params (DeltaSeconds :type "Float (single-precision)"))
  (`self.AddMovementInput` (`self.GetActorForwardVector`)))

(event `InputAction|Fire`
  (params (Key :type "Key Structure")))

(event `InputAxis|Pitch`
  (params (AxisValue :type "Float (single-precision)"))
  ; Pitch 회전
  (`self.K2_AddActorLocalRotation` (`KismetMathLibrary.MakeRotator` 0.0 (* AxisValue 60.0 (`GameplayStatics.GetWorldDeltaSeconds`)))))

(event `InputAxis|Roll`
  (params (AxisValue :type "Float (single-precision)"))
  ; Roll 회전
  (`self.K2_AddActorLocalRotation` (`KismetMathLibrary.MakeRotator` (* AxisValue 60.0 (`GameplayStatics.GetWorldDeltaSeconds`)))))

(fn `RotatePropeller`
  (params (Where :type "SceneComponent Object Reference") (RotationSpeed :type "Float (double-precision)"))
  (`SceneComponent.K2_AddLocalRotation` Where (`KismetMathLibrary.MakeRotator` (* RotationSpeed (`GameplayStatics.GetWorldDeltaSeconds`))) false false))

(fn `UserConstructionScript`)